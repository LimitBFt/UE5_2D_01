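; Player 1 character Kaguya, a 2D sprite fighter that moves on input and fires ranged or near attacks against actors tagged Usagi.
; It registers itself with the GameInstance, which supplies walk speed, attack stats and HP.
; Attacks are spawned through the ActorManager's pool along the last move direction, then a tinted cooldown blocks both movement input and attacking.
; Hits lower clamped HP, flash the sprite red, play a sound and trigger the HP check.
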(event Custom|MoveInput2
  (params (MoveValue :type Vector%202D%20Structure))
  (bind (_x _y) (Math|Vector2D|BreakVector2D MoveValue))
  ;[1 1 1] Move
  (if (not (Variables|Default|GetIsCoolDown_Kaguya))
    (bind _output_get (Variables|Default|SetXdirection _x))
    (bind _output_get_2 (Variables|Default|SetYdirection _y))
    (Variables|Default|SetCurrentMoveDirection_Kaguya (Math|Vector|MakeVector _output_get _output_get_2 0.0))
    (Pawn|Input|AddMovementInput "0.500000,0.000000,0.000000" (Variables|Default|GetXdirection) false)
    (Pawn|Input|AddMovementInput "0.000000,0.500000,0.000000" (Variables|Default|GetYdirection) false)))

(event Custom|23
  (params (IsRanged :type Boolean)))

(event Custom|Input_Attack_Kaguya
  (params (IsRanged :type Boolean))
  (bind _returnvalue (Transformation|GetActorLocation))
  (bind _as_game_instance_2d (Variables|Default|GetAs%20Game%20Instance%202D))
  (bind _as_game_instance_2d_2 (Variables|Default|GetAs%20Game%20Instance%202D))
  (bind _as_game_instance_2d_3 (Variables|Default|GetAs%20Game%20Instance%202D))
  (bind _currentmovedirection_kaguya (Variables|Default|GetCurrentMoveDirection_Kaguya))
  (bind _returnvalue_2 (Class|KismetMathLibrary|VectorNormal2D _currentmovedirection_kaguya 1e+01))
  (bind (_x _y) (Math|Vector|BreakVector _currentmovedirection_kaguya))
  (bind _actormanager (Variables|/Game/BP/GameInstance/GameInstance_2D.GameInstance_2D_C|GetActorManager _as_game_instance_2d))
  (bind _returnvalue_3 (Math|Trig|Atan2(Radians) _y _x))
  (bind _returnvalue_4 (* _returnvalue_2 2e+02))
  (bind _returnvalue_5 (Math|Trig|RadiansToDegrees _returnvalue_3))
  (bind _returnvalue_6 (+ _returnvalue _returnvalue_4))
  ;[1 1 1] Attack
  (Variables|Default|SetIs%20Ranged IsRanged)
  (if (not (Variables|Default|GetIsCoolDown_Kaguya))
    (if IsRanged
      (Default|SetAttackPoolKaguya _actormanager _returnvalue_6 "/Game/Chracter/Attack/Kaguya/Effect3/Anm_Kaguya_Effect3.Anm_Kaguya_Effect3" (Variables|/Game/BP/GameInstance/GameInstance_2D.GameInstance_2D_C|GetAttack_Damage_Kaguya_Far _as_game_instance_2d_2) (* _returnvalue_4 (Variables|/Game/BP/GameInstance/GameInstance_2D.GameInstance_2D_C|GetAttackdistance_Kaguya (Variables|Default|GetAs%20Game%20Instance%202D))) (Variables|/Game/BP/GameInstance/GameInstance_2D.GameInstance_2D_C|GetAttacksize_Kaguya_Far _as_game_instance_2d_2) (Variables|/Game/BP/GameInstance/GameInstance_2D.GameInstance_2D_C|GetAttackaoe_Kaguya_Far _as_game_instance_2d_2) "Usagi" 1e+01 (Math|Rotator|MakeRotator -9e+01 0.0 _returnvalue_5))
      (else
        (Default|SetAttackPoolKaguya _actormanager _returnvalue_6 "/Game/Chracter/Attack/Kaguya/Effect1/Attack1.Attack1" (Variables|/Game/BP/GameInstance/GameInstance_2D.GameInstance_2D_C|GetAttack_Damage_kaguya_Near _as_game_instance_2d_3) (* _returnvalue_4 "") (Variables|/Game/BP/GameInstance/GameInstance_2D.GameInstance_2D_C|GetAttacksize_Kaguya_Near _as_game_instance_2d_3) (Variables|/Game/BP/GameInstance/GameInstance_2D.GameInstance_2D_C|GetAttackaoe_Kaguya_Near _as_game_instance_2d_3) "Usagi" 1e+01 (Math|Rotator|MakeRotator -9e+01 0.0 _returnvalue_5))))
    (Variables|Default|SetIsCoolDown_Kaguya true)
    (Sprite|SetSpriteColor (Variables|Default|GetSprite) "(R=0.000000,G=0.658378,B=1.000000,A=1.000000)")
    (if (Variables|Default|GetIs%20Ranged)
      (Utilities|FlowControl|Delay (Variables|/Game/BP/GameInstance/GameInstance_2D.GameInstance_2D_C|GetCooldown_Kaguya_Far (Variables|Default|GetAs%20Game%20Instance%202D)))
      (else
        (Utilities|FlowControl|Delay (Variables|/Game/BP/GameInstance/GameInstance_2D.GameInstance_2D_C|GetCooldown_Kaguya_Near (Variables|Default|GetAs%20Game%20Instance%202D)))))
    (Sprite|SetSpriteColor (Variables|Default|GetSprite) "(R=1.000000,G=1.000000,B=1.000000,A=1.000000)")
    (Variables|Default|SetIsCoolDown_Kaguya false)))

(event EventBeginPlay
  (bind _asgame_instance_2d (CallFunction|GetGameInstance))
  ;[1 1 1] Game Instance
  (Variables|/Game/BP/GameInstance/GameInstance_2D.GameInstance_2D_C|SetKaguya _asgame_instance_2d self)
  (bind _output_get (Variables|Default|SetAs%20Game%20Instance%202D _asgame_instance_2d))
  (Variables|/Script/Engine.CharacterMovementComponent|SetMaxWalkSpeed (Variables|Character|GetCharacterMovement) (Variables|/Game/BP/GameInstance/GameInstance_2D.GameInstance_2D_C|GetWalkSpeed_Kaguya _output_get)))

(event Collision|EventActorBeginOverlap
  (params (OtherActor :type Actor%20Object%20Reference)))

(event EventTick
  (params (DeltaSeconds :type Float%20%28single-precision%29)))

(event EventHitDetectionKaguya
  (params (Damage%20Kaguya :type Float%20%28double-precision%29))
  (bind _as_game_instance_2d (Variables|Default|GetAs%20Game%20Instance%202D))
  ;[1 1 1] Hit Detection
  (Variables|/Game/BP/GameInstance/GameInstance_2D.GameInstance_2D_C|SetHP_Kaguya_Current _as_game_instance_2d (Math|Float|Clamp(Float) (- (Variables|/Game/BP/GameInstance/GameInstance_2D.GameInstance_2D_C|GetHP_Kaguya_Current _as_game_instance_2d) Damage%20Kaguya) 0.0 (Variables|/Game/BP/GameInstance/GameInstance_2D.GameInstance_2D_C|GetHP_Kaguya_Max _as_game_instance_2d)))
  (Sprite|SetSpriteColor (Variables|Default|GetSprite) "(R=1.000000,G=0.000000,B=0.000000,A=1.000000)")
  (Audio|PlaySound2D "/Game/Sound/Damage_Sound_1.Damage_Sound_1" 1.0 1.0 0.0 0 0)
  (Utilities|FlowControl|Delay 0.2)
  (Default|HPcheck (Variables|Default|GetAs%20Game%20Instance%202D))
  (Sprite|SetSpriteColor (Variables|Default|GetSprite) "(R=1.000000,G=1.000000,B=1.000000,A=1.000000)")
  (Development|PrintString (Utilities|String|ToString(Float) (Variables|/Game/BP/GameInstance/GameInstance_2D.GameInstance_2D_C|GetHP_Kaguya_Current _as_game_instance_2d))))

(fn ConstructionScript)