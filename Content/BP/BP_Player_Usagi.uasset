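; Player character Blueprint for Usagi, a 2D sprite fighter that moves, attacks targets tagged Kaguya, and takes damage.
; It registers itself on the game instance, then moves from input while storing the current direction to aim attacks.
; Attacks request pooled effects from the game instance's ActorManager: either a flying sword or a stationary, harder-hitting melee effect.
; Hits lower clamped HP, briefly flash the sprite red and print the remaining health.
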(event Custom|MoveInput1
  (params (MoveValue :type Vector%202D%20Structure))
  (bind (_x _y) (Math|Vector2D|BreakVector2D MoveValue))
  ;[1 1 1] Move
  (bind _output_get (Variables|Default|SetXdirection _x))
  (bind _output_get_2 (Variables|Default|SetYdirection _y))
  (Variables|Default|SetCurrentMoveDirection_Usagi (Math|Vector|MakeVector _output_get _output_get_2 0.0))
  (Pawn|Input|AddMovementInput "0.500000,0.000000,0.000000" (Variables|Default|GetXdirection) false)
  (Pawn|Input|AddMovementInput "0.000000,0.500000,0.000000" (Variables|Default|GetYdirection) false))

(event Custom|Input_Attack_Usagi
  (params (IsRanged :type Boolean%20%28by%20ref%29))
  (bind _returnvalue (Transformation|GetActorLocation))
  (bind _as_game_instance_2d (Variables|Default|GetAs%20Game%20Instance%202D))
  (bind _currentmovedirection_usagi (Variables|Default|GetCurrentMoveDirection_Usagi))
  (bind _currentmovedirection_usagi_2 (Variables|Default|GetCurrentMoveDirection_Usagi))
  (bind _returnvalue_2 (Class|KismetMathLibrary|VectorNormal2D _currentmovedirection_usagi 1e+01))
  (bind (_x _y) (Math|Vector|BreakVector _currentmovedirection_usagi_2))
  (bind _actormanager (Variables|/Game/BP/GameInstance/GameInstance_2D.GameInstance_2D_C|GetActorManager _as_game_instance_2d))
  (bind _returnvalue_3 (Math|Trig|Atan2(Radians) _y _x))
  (bind _returnvalue_4 (* _returnvalue_2 2e+02))
  (bind _returnvalue_5 (Math|Trig|RadiansToDegrees _returnvalue_3))
  (bind _returnvalue_6 (+ _returnvalue _returnvalue_4))
  ;[1 1 1] Attack
  (if IsRanged
    (Default|SetAttackPoolUsagi _actormanager _returnvalue_6 "/Game/Chracter/Attack/Usagi/Sword_fly/sword_fly.sword_fly" 1.0 (* _returnvalue_4 (Variables|Default|GetAttackdistance_Usagi)) "0.900000,0.900000,0.900000" "0.600000,0.600000,0.600000" "Kaguya" 1e+01 (Math|Rotator|MakeRotator -9e+01 0.0 _returnvalue_5))
    (else
      (Default|SetAttackPoolUsagi _actormanager _returnvalue_6 "/Game/Chracter/Attack/Usagi/Sword_Kinsetu/Anm_Usagi_Effect_1.Anm_Usagi_Effect_1" 2.0 (* _returnvalue_4 "") "0.900000,0.900000,0.900000" "0.600000,0.600000,0.600000" "Kaguya" 1e+01 (Math|Rotator|MakeRotator -9e+01 0.0 _returnvalue_5)))))

(event EventHitDetectionUsagi
  (params (Damage%20Usagi :type Float%20%28double-precision%29))
  ;[1 1 1] Hit Detection
  (Variables|Default|SetHP_Usagi_Current (Math|Float|Clamp(Float) (- (Variables|Default|GetHP_Usagi_Current) Damage%20Usagi) 0.0 (Variables|Default|GetHP_Usagi_Max)))
  (Sprite|SetSpriteColor (Variables|Default|GetSprite) "(R=1.000000,G=0.000000,B=0.024068,A=1.000000)")
  (Utilities|FlowControl|Delay 0.2)
  (Sprite|SetSpriteColor (Variables|Default|GetSprite) "(R=1.000000,G=1.000000,B=1.000000,A=1.000000)")
  (Development|PrintString (Utilities|String|ToString(Float) (Variables|Default|GetHP_Usagi_Current))))

(event Collision|EventActorBeginOverlap
  (params (OtherActor :type Actor%20Object%20Reference)))

(event EventTick
  (params (DeltaSeconds :type Float%20%28single-precision%29)))

(event EventBeginPlay
  (bind _asgame_instance_2d (CallFunction|GetGameInstance))
  ;[1 1 1] Set Game Instance
  (Variables|/Game/BP/GameInstance/GameInstance_2D.GameInstance_2D_C|SetUsagi _asgame_instance_2d self)
  (Variables|Default|SetAs%20Game%20Instance%202D _asgame_instance_2d))

(fn ConstructionScript)